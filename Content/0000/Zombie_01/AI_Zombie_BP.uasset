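; Zombie AI pawn that chases the first FirstPersonCharacter found in the level and is destroyed by its TakeDamage event.
; After a short BeginPlay delay it caches that character and starts a movement loop that runs AI MoveTo while CanMove is set.
; The loop retries after a delay, longer on success than on failure or when movement is disabled.
; A separate StopMovement event halts the current movement immediately.
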(event `self.ReceiveBeginPlay`
  (`KismetSystemLibrary.Delay` 0.2)
  (bind _outactors (`GameplayStatics.GetAllActorsOfClass` "/Game/0000/FirstPersonCharacter.FirstPersonCharacter_C"))
  (set `self.PlayerCharacter` (`|GetArrayItem` _outactors))
  (`self.Movement_Loop`))

(event `StopMovement`
  (`MovementComponent.StopMovementImmediately` (`self.CharacterMovement`)))

(event `Movement_Loop`
  (if (`self.CanMove`) :!label _label
    (bind _movementresult (`|AIMoveTo` self (0.0 0.0 0.0) (`self.PlayerCharacter`) 50.0 true)
      (:`OnSuccess`
        _)
      (:`OnFail`
        _))
    (switch `EPathFollowingResult` _movementresult
      (:`Success`
        (`KismetSystemLibrary.Delay` 1.5)
        (goto _label))
      (:`Blocked`
        _)
      (:`OffPath`
        _)
      (:`Aborted`
        _)
      (:`Invalid`
        _)))
  (`KismetSystemLibrary.Delay` 0.5)
  (goto _label))

(event `TakeDamage`
  (`self.K2_DestroyActor`))

(fn `UserConstructionScript`)